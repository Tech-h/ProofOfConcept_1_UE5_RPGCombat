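; Heavy knight enemy that chases the player with AIMoveTo and attacks on arrival, retrying after a delay if the move fails.
; Swings damage the player when a forward line trace hits anything; every fourth attack plays a double spin montage with no damage logic.
; Damage lowers Health; at zero it plays a slowed death montage, then moves the capsule far away and calls SpawnActor.
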(event Custom|ChasePlayer
  (bind _returnvalue (Game|GetPlayerCharacter 0))
  (if (Variables|Default|GetNotSpinAttacking)
    (AI|AIMoveTo self (Transformation|GetActorLocation _returnvalue) _returnvalue 1e+01 false
      (:OnSuccess
        (CallFunction|OverheadAttack))
      (:OnFail
        (Utilities|FlowControl|Delay 3.0)
        (CallFunction|ChasePlayer)))))

(event Custom|OverheadAttack
  (bind _capsulecomponent (Variables|Collision|GetCapsuleComponent))
  (bind _returnvalue (Transformation|GetWorldLocation _capsulecomponent))
  (bind _returnvalue_2 (Math|Vector|GetForwardVector _capsulecomponent))
  (Variables|Default|Sethits (+ (Variables|Default|Gethits) 1))
  (if (== (Variables|Default|Gethits) 4)
    (Variables|Default|Sethits 0)
    (Animation|Montage|PlayMontage (Variables|Character|GetMesh) "/Game/Characters/HeavyKnight/HK_Animations/HK_Animations_metarig_SpinAttack_Montage.HK_Animations_metarig_SpinAttack_Montage" 2.0
      (:OnBlendOut
        (Animation|Montage|PlayMontage (Variables|Character|GetMesh) "/Game/Characters/HeavyKnight/HK_Animations/HK_Animations_metarig_SpinAttack_Montage.HK_Animations_metarig_SpinAttack_Montage" 2.0
          (:OnCompleted
            (CallFunction|ChasePlayer)))))
    (elif (Variables|Default|GetNotSpinAttacking)
      (Animation|Montage|PlayMontage (Variables|Character|GetMesh) "/Game/Characters/HeavyKnight/HK_Animations/HK_Animations_metarig_SwingAttack_Montage.HK_Animations_metarig_SwingAttack_Montage" 1.5
        (:OnBlendOut
          (bind _returnvalue_3 (Collision|LineTraceByChannel _returnvalue (+ _returnvalue (* _returnvalue_2 3e+02)) "TraceTypeQuery1" false 0 "Persistent"))
          (if _returnvalue_3
            (bind _asbp_player_character (Utilities|Casting|CastToBP_PlayerCharacter (Game|GetPlayerCharacter 0)))
            (Default|Damage _asbp_player_character 3e+01 _returnvalue_2))
          (CallFunction|ChasePlayer))))))

(event EventBeginPlay
  (CallFunction|ChasePlayer))

(event EventDamage
  (params (Damage :type Float%20%28double-precision%29) (Hit%20Location :type Vector :default "0, 0, 0"))
  (bind _output_get (Variables|Default|SetHealth (- (Variables|Default|GetHealth) Damage)))
  (if (<= (Variables|Default|GetHealth) 0.0)
    (Components|Movement|StopMovementImmediately (Variables|Character|GetCharacterMovement))
    (Animation|Montage|PlayMontage (Variables|Character|GetMesh) "/Game/Characters/HeavyKnight/HK_Animations/HK_KnightDeath_metarig_Die_Montage.HK_KnightDeath_metarig_Die_Montage" 0.2
      (:OnBlendOut
        (Components|MoveComponentTo (Variables|Collision|GetCapsuleComponent) "20000.000000,2000.000000,20000.000000" "0, 0, 0" false false 0.2 false)
        (Game|SpawnActorfromClass "/Game/Characters/SquidBoss/BP_Squid.BP_Squid_C" (Math|Transform|MakeTransform "1000.000000,0.000000,0.000000" "0, 0, 0" "1.000000,1.000000,1.000000") "Undefined" "MultiplyWithRoot" 0 0)))
    (else
      (Development|PrintString (Utilities|String|ToString(Float) _output_get)))))

(fn ConstructionScript)